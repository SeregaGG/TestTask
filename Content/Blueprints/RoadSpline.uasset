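; RoadSpline is a Blueprint that lays spline mesh segments along a spline, apparently to form a road.
; The construction script divides the spline length by Divisor and adds a SplineMeshComponent at each interval, with an inclusive loop covering the remainder.
; Each segment takes local-space start and end locations from the spline, with tangents built from its direction scaled by NewVar0.
; The event graph holds no active logic.
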(fn `UserConstructionScript`
  (bind _spline (`self.Spline`))
  (bind _divisor (`self.Divisor`))
  (for _index (range (+ (`.ReturnValue` (`KismetMathLibrary.FMod` (`SplineComponent.GetSplineLength` (`self.Spline`)) (`self.Divisor`))) 1))
    (bind _returnvalue (`AddComponent|NODE_AddSplineMeshComponent-0`))
    (bind _returnvalue_2 (* _index _divisor))
    (bind _returnvalue_3 (+ _returnvalue_2 _divisor))
    (`SplineMeshComponent.SetStartAndEnd` _returnvalue (`SplineComponent.GetLocationAtDistanceAlongSpline` _spline _returnvalue_2 "Local") (* (`SplineComponent.GetDirectionAtDistanceAlongSpline` _spline _returnvalue_2 "Local") (`self.NewVar_0`)) (`SplineComponent.GetLocationAtDistanceAlongSpline` _spline _returnvalue_3 "Local") (* (`SplineComponent.GetDirectionAtDistanceAlongSpline` _spline _returnvalue_3 "Local") (`self.NewVar_0`)) true)))